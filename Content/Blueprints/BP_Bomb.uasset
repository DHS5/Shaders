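; BP_Bomb is a short-lived area-effect bomb actor that deals fire damage to enemies it overlaps.
; Each tick it multiplies a stored scale by GrowRate and applies it to its Sphere component until the X scale exceeds one.
; Overlapping a BP_Enemy calls that enemy's FireDamage.
; The actor destroys itself after a fixed delay from BeginPlay.
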(event `self.ReceiveActorBeginOverlap`
  (params (OtherActor :type "Actor Object Reference"))
  (bind _asbp_enemy (cast `/Game/Blueprints/Enemies/BP_Enemy` OtherActor))
  (`/Game/Blueprints/Enemies/BP_Enemy.Fire Damage` _asbp_enemy))

(event `self.ReceiveBeginPlay`
  (`KismetSystemLibrary.Delay` 5.0)
  (`self.K2_DestroyActor`))

(event `self.ReceiveTick`
  (params (DeltaSeconds :type "Float (single-precision)"))
  (bind _old_scale_x (`KismetMathLibrary.BreakVector` (`self.old scale`)))
  (if (not (> _old_scale_x 1.0))
    (bind _output_get (set `self.old scale` (* (`self.old scale`) (`self.grow rate`))))
    (`SceneComponent.SetRelativeScale3D` (`self.Sphere`) _output_get)))

(fn `UserConstructionScript`)