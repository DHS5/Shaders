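; BP_FireBall is a short-lived fireball actor that calls FireDamage on any BP_Enemy it overlaps and destroys itself five seconds after spawning.
; BeginPlay creates a dynamic material on the Sphere and sets its Direction parameter to the reversed forward vector.
; Tick drives the material's Length from the summed absolute velocity components, scaled down.
; The high-speed branch adds a zero impulse, so it has no effect on motion.
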(event `self.ReceiveActorBeginOverlap`
  (params (OtherActor :type "Actor Object Reference"))
  (bind _asbp_enemy (cast `/Game/Blueprints/Enemies/BP_Enemy` OtherActor))
  (`/Game/Blueprints/Enemies/BP_Enemy.Fire Damage` _asbp_enemy))

(event `self.ReceiveBeginPlay`
  (bind _sphere (`self.Sphere`))
  (bind _returnvalue (`PrimitiveComponent.CreateDynamicMaterialInstance` _sphere 0 null "None"))
  (bind _output_get (set `self.MI` _returnvalue))
  (`MaterialInstanceDynamic.SetVectorParameterValue` _output_get "Direction" (`KismetMathLibrary.Conv_VectorToLinearColor` (* (`SceneComponent.GetForwardVector` _sphere) (-1.0 -1.0 -1.0))))
  (`KismetSystemLibrary.Delay` 5.0)
  (`self.K2_DestroyActor`))

(event `self.ReceiveTick`
  (params (DeltaSeconds :type "Float (single-precision)"))
  (bind (_returnvalue_x _returnvalue_y _returnvalue_z) (`KismetMathLibrary.BreakVector` (`SceneComponent.GetComponentVelocity` (`self.Sphere`))))
  (bind _returnvalue (* (+ (+ (`KismetMathLibrary.Abs` _returnvalue_x) (`KismetMathLibrary.Abs` _returnvalue_y)) (`KismetMathLibrary.Abs` _returnvalue_z)) 0.1))
  (if (> _returnvalue 100.0)
    (`PrimitiveComponent.AddImpulse` (`self.Sphere`) (0.0 0.0 0.0) "None" false))
  (`MaterialInstanceDynamic.SetScalarParameterValue` (`self.MI`) "Length" _returnvalue))

(fn `UserConstructionScript`)